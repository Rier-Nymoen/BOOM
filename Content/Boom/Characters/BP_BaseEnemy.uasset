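; Base enemy Blueprint that registers its AI controller's team for perception when play begins.
; On BeginPlay it casts and caches its BOOMAIController, sets the generic team ID to TeamOne, then requests a perception stimuli listener update so the new affiliation takes effect.
; A debug print confirms the assignment, and the construction script only calls its parent.
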(event `self.ReceiveBeginPlay`
  (bind _asboomaicontroller (cast `BOOMAIController` (`self.GetController` self)))
  (bind _output_get (set `self.As BOOMAIController` _asboomaicontroller))
  (`BOOMAIController.SetGenericTeamId` _output_get (`self.TeamOne`))
  (`AIPerceptionComponent.RequestStimuliListenerUpdate` (`BOOMAIController.AIPerceptionComponent` _asboomaicontroller))
  (`KismetSystemLibrary.PrintString` "Team Set"))

(fn `UserConstructionScript`
  (`parent.UserConstructionScript`))